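; Grenade actor that explodes on a fixed fuse after spawning and damages actors tagged Enemy.
; BeginPlay waits out the fuse, plays explosion particles and sound at the Sphere, hides the mesh and opens a short CanHit window before destroying itself.
; The GrenadeDamage component applies damage only on begin-overlap events during that window, so enemies already inside at detonation are not hit unless they re-enter.
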(event OnComponentBeginOverlap(GrenadeDamage)
  (params (OverlappedComponent :type Primitive%20Component%20Object%20Reference) (OtherActor :type Actor%20Object%20Reference) (OtherComp :type Primitive%20Component%20Object%20Reference) (OtherBodyIndex :type Integer) (bFromSweep :type Boolean) (SweepResult :type Hit%20Result%20Structure%20%28by%20ref%29))
  (if (and (Actor|ActorHasTag OtherActor "Enemy") (Variables|Default|GetCanHit?))
    (Game|Damage|ApplyDamage OtherActor 4e+01 0 self)))

(event EventBeginPlay
  (Utilities|FlowControl|Delay 5.0)
  (Effects|SpawnEmitteratLocation "/Game/StarterContent/Particles/P_Explosion.P_Explosion" (Transformation|GetWorldLocation (Variables|Default|GetSphere)))
  (Audio|PlaySoundatLocation "/Game/StarterContent/Audio/Explosion_Cue.Explosion_Cue" (Transformation|GetWorldLocation (Variables|Default|GetSphere)) "0, 0, 0" 1.0 1.0 0.0 0 0 0 0)
  (Variables|Default|SetCanHit? true)
  (Development|SetHiddeninGame (Variables|Default|GetMesh) true false)
  (Utilities|FlowControl|Delay 3.0)
  (Variables|Default|SetCanHit? false)
  (Actor|DestroyActor))

(event Collision|EventActorBeginOverlap
  (params (OtherActor :type Actor%20Object%20Reference)))

(event EventTick
  (params (DeltaSeconds :type Float%20%28single-precision%29)))

(fn ConstructionScript)