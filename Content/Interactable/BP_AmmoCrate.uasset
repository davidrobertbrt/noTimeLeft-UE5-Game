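; BP_AmmoCrate is an interactable pickup that refills the player's ammo and grenades and restores some health, capped at full.
; A box overlap with BP_PlayableCharacter enables input and opens a gate; leaving disables input and closes it.
; The INP_InteractWith action passes through that gate, applies the rewards to player character 0, then destroys the crate, making it single-use.
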(event OnComponentBeginOverlap(Box)
  (params (OverlappedComponent :type Primitive%20Component%20Object%20Reference) (OtherActor :type Actor%20Object%20Reference) (OtherComp :type Primitive%20Component%20Object%20Reference) (OtherBodyIndex :type Integer) (bFromSweep :type Boolean) (SweepResult :type Hit%20Result%20Structure%20%28by%20ref%29))
  (Utilities|Casting|CastToBP_PlayableCharacter OtherActor)
  (Input|EnableInput (Game|GetPlayerController 0))
  (Utilities|FlowControl|Gate true) ; enters at Open
)

(event OnComponentEndOverlap(Box)
  (params (OverlappedComponent :type Primitive%20Component%20Object%20Reference) (OtherActor :type Actor%20Object%20Reference) (OtherComp :type Primitive%20Component%20Object%20Reference) (OtherBodyIndex :type Integer))
  (Utilities|Casting|CastToBP_PlayableCharacter OtherActor)
  (Input|DisableInput (Game|GetPlayerController 0))
  (Utilities|FlowControl|Gate true) ; enters at Close
)

(event Input|EnhancedActionEvents|EnhancedInputActionINP_InteractWith
  (params (ActionValue :type Boolean) (ElapsedSeconds :type Float%20%28double-precision%29) (TriggeredSeconds :type Float%20%28double-precision%29) (InputAction :type Input%20Action%20Object%20Reference :default "/Game/PlayableCharacter/Input/Actions/INP_InteractWith.INP_InteractWith"))
  (Utilities|FlowControl|Gate true
    (:Exit
      (bind _asbp_playable_character (Utilities|Casting|CastToBP_PlayableCharacter (Game|GetPlayerCharacter 0)))
      (Variables|/Game/PlayableCharacter/BP_PlayableCharacter.BP_PlayableCharacter_C|SetAmmo _asbp_playable_character (+ (Variables|/Game/PlayableCharacter/BP_PlayableCharacter.BP_PlayableCharacter_C|GetAmmo _asbp_playable_character) 30))
      (Variables|/Game/PlayableCharacter/BP_PlayableCharacter.BP_PlayableCharacter_C|SetGrenadeAmmo _asbp_playable_character (+ (Variables|/Game/PlayableCharacter/BP_PlayableCharacter.BP_PlayableCharacter_C|GetGrenadeAmmo _asbp_playable_character) 2))
      (Variables|/Game/PlayableCharacter/BP_PlayableCharacter.BP_PlayableCharacter_C|SetHealth _asbp_playable_character (Math|Float|Clamp(Float) (+ (Variables|/Game/PlayableCharacter/BP_PlayableCharacter.BP_PlayableCharacter_C|GetHealth _asbp_playable_character) 15.0) 0.0 1e+02))
      (Actor|DestroyActor))))

(event EventBeginPlay)

(event Collision|EventActorBeginOverlap
  (params (OtherActor :type Actor%20Object%20Reference)))

(event EventTick
  (params (DeltaSeconds :type Float%20%28single-precision%29)))

(fn ConstructionScript)