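; BP_MainHUD is the player's HUD Blueprint, managing the ammo and kill score widgets on screen.
; On BeginPlay it creates both widgets, stores references to them and adds them to the viewport.
; The PlayerDead event removes both stored widgets from their parent.
; A separate RemoveHud function removes all top-level widgets of a given class.
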(event Custom|PlayerDead
  (Widget|RemovefromParent (Variables|Default|GetKillWidget))
  (Widget|RemovefromParent (Variables|Default|GetAmmoWidget)))

(event EventBeginPlay
  (bind _returnvalue (UserInterface|CreateWidget "/Game/PlayableCharacter/BP_AmmoWidget.BP_AmmoWidget_C"))
  (bind _output_get (Variables|Default|SetAmmoWidget _returnvalue))
  (UserInterface|Viewport|AddtoViewport _output_get 0)
  (bind _returnvalue_2 (UserInterface|CreateWidget "/Game/PlayableCharacter/BP_KillScoreWidget.BP_KillScoreWidget_C"))
  (bind _output_get_2 (Variables|Default|SetKillWidget _returnvalue_2))
  (UserInterface|Viewport|AddtoViewport _output_get_2 0))

(event Collision|EventActorBeginOverlap
  (params (OtherActor :type Actor%20Object%20Reference)))

(event EventTick
  (params (DeltaSeconds :type Float%20%28single-precision%29)))

(fn ConstructionScript)

(fn RemoveHud
  (params (Widget%20Class :type User%20Widget%20Class%20Reference))
  (bind _foundwidgets (Widget|GetAllWidgetsOfClass Widget%20Class true))
  (Widget|RemovefromParent _foundwidgets))