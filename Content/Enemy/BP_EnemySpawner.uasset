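; Enemy spawner actor that repeatedly spawns batches of a configurable enemy class at its own transform while the game mode's alive count is below its maximum.
; BeginPlay spawns the first batch unconditionally and caches BP_ThirdPersonGameMode.
; After each SpawnDelay, SpawnEnemy re-triggers itself if EnemiesAlive is under MaxEnemies.
; Otherwise CheckShouldSpawn polls at the same interval until room opens, forming an endless delay-based event loop.
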(event Custom|SpawnEnemy
  (params (Enemy :type Actor%20Class%20Reference) (SpawnTransform :type Transform) (NumberOfEnemies :type Integer))
  (bind _gamemoderef (Variables|Default|GetGameModeRef))
  (for _index (range 0 (- NumberOfEnemies 1))
    (Game|SpawnActorfromClass Enemy SpawnTransform "Undefined" "MultiplyWithRoot" 0 0))
  (Utilities|FlowControl|Delay (Variables|Default|GetSpawnDelay))
  (if (< (Variables|/Game/ThirdPerson/Blueprints/BP_ThirdPersonGameMode.BP_ThirdPersonGameMode_C|GetEnemiesAlive _gamemoderef) (Variables|/Game/ThirdPerson/Blueprints/BP_ThirdPersonGameMode.BP_ThirdPersonGameMode_C|GetMaxEnemies _gamemoderef))
    (CallFunction|SpawnEnemy (Variables|Default|GetEnemy) (Transformation|GetActorTransform) (Variables|Default|GetNumber%20Of%20Enemies))
    (else
      (CallFunction|CheckShouldSpawn))))

(event Custom|Check%20should%20spawn
  (bind _gamemoderef (Variables|Default|GetGameModeRef))
  (Utilities|FlowControl|Delay (Variables|Default|GetSpawnDelay))
  (if (< (Variables|/Game/ThirdPerson/Blueprints/BP_ThirdPersonGameMode.BP_ThirdPersonGameMode_C|GetEnemiesAlive _gamemoderef) (Variables|/Game/ThirdPerson/Blueprints/BP_ThirdPersonGameMode.BP_ThirdPersonGameMode_C|GetMaxEnemies _gamemoderef))
    (CallFunction|SpawnEnemy (Variables|Default|GetEnemy) (Transformation|GetActorTransform) (Variables|Default|GetNumber%20Of%20Enemies))
    (else
      (CallFunction|CheckShouldSpawn))))

(event EventBeginPlay
  (Utilities|FlowControl|Sequence
    (:then_0
      (CallFunction|SpawnEnemy (Variables|Default|GetEnemy) (Transformation|GetActorTransform) (Variables|Default|GetNumber%20Of%20Enemies)))
    (:then_1
      (bind _asbp_third_person_game_mode (Utilities|Casting|CastToBP_ThirdPersonGameMode (Game|GetGameMode)))
      (Variables|Default|SetGameModeRef _asbp_third_person_game_mode))))

(fn ConstructionScript)