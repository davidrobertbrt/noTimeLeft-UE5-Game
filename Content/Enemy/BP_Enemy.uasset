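; Enemy character that endlessly chases the player with AI MoveTo at a random walk speed and punches on contact.
; Damage updates a health widget, shown only while the player is within a trigger, and pauses movement for a random hit montage.
; At zero health it plays a death montage, credits the player's kill score, may drop a ground-traced ammo crate, notifies the game mode and is destroyed after a delay.
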(event OnComponentBeginOverlap(SeeHealthWidget)
  (params (OverlappedComponent :type Primitive%20Component%20Object%20Reference) (OtherActor :type Actor%20Object%20Reference) (OtherComp :type Primitive%20Component%20Object%20Reference) (OtherBodyIndex :type Integer) (bFromSweep :type Boolean) (SweepResult :type Hit%20Result%20Structure%20%28by%20ref%29))
  (Utilities|Casting|CastToBP_PlayableCharacter OtherActor)
  (Rendering|SetVisibility (Variables|Default|GetHealthWidget) true false))

(event OnComponentEndOverlap(SeeHealthWidget)
  (params (OverlappedComponent :type Primitive%20Component%20Object%20Reference) (OtherActor :type Actor%20Object%20Reference) (OtherComp :type Primitive%20Component%20Object%20Reference) (OtherBodyIndex :type Integer))
  (Utilities|Casting|CastToBP_PlayableCharacter OtherActor)
  (Rendering|SetVisibility (Variables|Default|GetHealthWidget) false false))

(event Custom|ChasePlayer
  (params (Player%20To%20Chase :type BP%20Playable%20Character%20Object%20Reference))
  (if (not (Variables|Default|GetIsDead))
    (AI|AIMoveTo self "0, 0, 0" Player%20To%20Chase 5.0 false
      (:OnSuccess
        _)
      (:OnFail
        _))
    (CallFunction|ChasePlayer (Variables|Default|GetCharacter%20Ref))))

(event EventBeginPlay
  (bind _asbp_playable_character (Utilities|Casting|CastToBP_PlayableCharacter (Game|GetPlayerCharacter 0)))
  (bind _output_get (Variables|Default|SetCharacter%20Ref _asbp_playable_character))
  (CallFunction|ChasePlayer _output_get)
  (Variables|/Script/Engine.CharacterMovementComponent|SetMaxWalkSpeed (Variables|Character|GetCharacterMovement) (Utilities|Select :Index (Math|Random|RandomInteger 3) :Option%200 2e+02 :Option%201 2.5e+02 :Option%202 3e+02 :Option%203 3.5e+02))
  (bind _asbp_health_enemy_widget (Utilities|Casting|CastToBP_HealthEnemyWidget (UserInterface|GetUserWidgetObject (Variables|Default|GetHealthWidget))))
  (Variables|Default|SetHealthWidgetRef _asbp_health_enemy_widget)
  (bind _asbp_third_person_game_mode (Utilities|Casting|CastToBP_ThirdPersonGameMode (Game|GetGameMode)))
  (Default|SpawnEnemies _asbp_third_person_game_mode))

(event Collision|EventActorBeginOverlap
  (params (OtherActor :type Actor%20Object%20Reference)))

(event Game|Damage|EventAnyDamage
  (params (Damage :type Float%20%28single-precision%29) (DamageType :type Damage%20Type%20Object%20Reference) (InstigatedBy :type Controller%20Object%20Reference) (DamageCauser :type Actor%20Object%20Reference))
  (bind _returnvalue (Transformation|GetActorLocation))
  (bind _returnvalue_2 (Transformation|GetActorLocation))
  (if (not (Variables|Default|GetIsDead))
    (bind _output_get (Variables|Default|SetHealth (Math|Float|Clamp(Float) (- (Variables|Default|GetHealth) Damage) 0.0 1e+02)))
    (Variables|/Game/Enemy/BP_HealthEnemyWidget.BP_HealthEnemyWidget_C|SetHealthStatus (Variables|Default|GetHealthWidgetRef) _output_get)
    (if (== _output_get 0.0)
      (Audio|PlaySoundatLocation "/Game/SFX/Character/Death/Death_Cue.Death_Cue" _returnvalue "0, 0, 0" 1.0 1.0 0.0 0 0 0 0)
      (Utilities|FlowControl|Sequence
        (:then_0
          (bind _asbp_playable_character (Utilities|Casting|CastToBP_PlayableCharacter (Game|GetPlayerCharacter 0)))
          (Math|Integer|IncrementInt (Variables|/Game/PlayableCharacter/BP_PlayableCharacter.BP_PlayableCharacter_C|GetKillScore _asbp_playable_character)
            (:%20%20
              (if (Math|Random|RandomBoolwithWeight 0.5)
                (bind _outhit (Collision|LineTraceByChannel _returnvalue_2 (- _returnvalue_2 "0.000000,0.000000,1500.000000") "TraceTypeQuery1" false 0 "None"))
                (Game|SpawnActorfromClass "/Game/Interactable/BP_AmmoCrate.BP_AmmoCrate_C" (Math|Transform|MakeTransform (.Location (Collision|BreakHitResult _outhit)) "0, 0, 0" "1.000000,1.000000,1.000000") "Undefined" "MultiplyWithRoot" 0 0)))))
        (:then_1
          (Utilities|FlowControl|Delay 6e+01)
          (Actor|DestroyActor))
        (:then_2
          (Pawn|Components|CharacterMovement|DisableMovement (Variables|Character|GetCharacterMovement))
          (Variables|Default|SetIsDead true)
          (Animation|PlayAnimMontage (Utilities|Select :Index (Math|Random|RandomInteger 3) :Option%200 "/Game/Enemy/Animations/Death_1_Montage.Death_1_Montage" :Option%201 "/Game/Enemy/Animations/Death_2_Montage.Death_2_Montage" :Option%202 "/Game/Enemy/Animations/Death_3_Montage.Death_3_Montage" :Option%203 "/Game/Enemy/Animations/Death_4_Montage.Death_4_Montage") 1.0 "None")
          (Collision|SetCollisionEnabled (Variables|Collision|GetCapsuleComponent) "NoCollision"))
        (:then_3
          (bind _asbp_third_person_game_mode (Utilities|Casting|CastToBP_ThirdPersonGameMode (Game|GetGameMode)))
          (Default|KillEnemy _asbp_third_person_game_mode)))
      (else
        (Audio|PlaySoundatLocation "/Game/SFX/Character/Damage/Cue_Damage.Cue_Damage" _returnvalue "0, 0, 0" 1.0 1.0 0.0 0 0 0 0)
        (Utilities|FlowControl|Sequence
          (:then_0
            (Pawn|Components|CharacterMovement|DisableMovement (Variables|Character|GetCharacterMovement))
            (bind _returnvalue_3 (Animation|PlayAnimMontage (Utilities|Select :Index (Math|Random|RandomInteger 3) :Option%200 "/Game/Enemy/Animations/Hit_1_Montage.Hit_1_Montage" :Option%201 "/Game/Enemy/Animations/Hit_2_Montage.Hit_2_Montage" :Option%202 "/Game/Enemy/Animations/Hit_3_Montage.Hit_3_Montage" :Option%203 "/Game/Enemy/Animations/Hit_4_Montage.Hit_4_Montage") 1.0 "None"))
            (Utilities|FlowControl|Delay _returnvalue_3)
            (if (not (Variables|Default|GetIsDead))
              (Pawn|Components|CharacterMovement|SetMovementMode (Variables|Character|GetCharacterMovement) "MOVE_Walking" 0))))))))

(event Collision|EventHit
  (params (MyComp :type Primitive%20Component%20Object%20Reference) (Other :type Actor%20Object%20Reference) (OtherComp :type Primitive%20Component%20Object%20Reference) (bSelfMoved :type Boolean) (HitLocation :type Vector :default "0, 0, 0") (HitNormal :type Vector :default "0, 0, 0") (NormalImpulse :type Vector :default "0, 0, 0") (Hit :type Hit%20Result%20Structure%20%28by%20ref%29))
  (if (and (not (Variables|Default|GetIsDead)) (Actor|ActorHasTag Other "Player"))
    (Pawn|Components|CharacterMovement|DisableMovement (Variables|Character|GetCharacterMovement))
    (Game|Damage|ApplyDamage (Variables|Default|GetCharacter%20Ref) 15.0 0 self)
    (bind _returnvalue (Animation|PlayAnimMontage "/Game/Enemy/Animations/HitPlayer/Montage_Punching.Montage_Punching" 1.0 "None"))
    (Utilities|FlowControl|Delay _returnvalue)
    (Pawn|Components|CharacterMovement|SetMovementMode (Variables|Character|GetCharacterMovement) "MOVE_Walking" 0)))

(fn ConstructionScript)